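; Actor component that tracks stamina for sprinting, judging by its name and variables.
; Each tick it drains CurrentStamina while IsSprinting is true and regenerates it otherwise, scaled by delta time and clamped between zero and MaxStamina.
; IsSprinting is only read here, and the current value prints every frame as debug output.
; UpdateStaminaDisplay is an empty stub.
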(event EventBeginPlay)

(event EventTick
  (params (DeltaSeconds :type Float%20%28single-precision%29))
  (Development|PrintString (Utilities|String|ToString(Float) (Variables|Default|GetCurrentStamina)) true false)
  (if (Variables|Default|GetbIsSprinting)
    (Variables|Default|SetCurrentStamina (Math|Float|Max(Float) (- (Variables|Default|GetCurrentStamina) (* (Variables|Default|GetStaminaDepletionRate) DeltaSeconds)) 0.0))
    (else
      (Variables|Default|SetCurrentStamina (Math|Float|Min(Float) (+ (Variables|Default|GetCurrentStamina) (* DeltaSeconds (Variables|Default|GetStaminaRegenRate))) (Variables|Default|GetMaxStamina))))))

(fn UpdateStaminaDisplay)