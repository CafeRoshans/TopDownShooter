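; Door Blueprint that slides its mesh upward while a Character stands in the door trigger, with a sound and an impact effect on entry.
; Tick raises the relative Z at Speed until it reaches a fixed height and flags it fully open; leaving pauses it, with no closing logic.
; A separate exit trigger only prints a "Door" message when a Character is inside and the door is fully open.
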(event OnComponentBeginOverlap(DoorTrigger)
  (params (OverlappedComponent :type Primitive%20Component%20Object%20Reference) (OtherActor :type Actor%20Object%20Reference) (OtherComp :type Primitive%20Component%20Object%20Reference) (OtherBodyIndex :type Integer) (bFromSweep :type Boolean) (SweepResult :type Hit%20Result%20Structure%20%28by%20ref%29))
  (bind _door (Variables|Default|GetDoor))
  (bind _relativelocation (Variables|/Script/Engine.SceneComponent|GetRelativeLocation _door))
  (Utilities|Casting|CastToCharacter OtherActor)
  (Variables|Default|SetbIsOpening true)
  (Audio|SpawnSoundatLocation "/Game/Free_Sounds_Pack/cue/Wood_Move_2-1_Cue.Wood_Move_2-1_Cue" (Math|Vector|MakeVector (.x _relativelocation) (.y _relativelocation) (.z _relativelocation)) "0, 0, 0" 1.0 1.0 0.0 0 0)
  (Components|Activation|SetActive (Variables|Default|GetNS_Big_Hammer_Impact) true false))

(event OnComponentEndOverlap(DoorTrigger)
  (params (OverlappedComponent :type Primitive%20Component%20Object%20Reference) (OtherActor :type Actor%20Object%20Reference) (OtherComp :type Primitive%20Component%20Object%20Reference) (OtherBodyIndex :type Integer))
  (Utilities|Casting|CastToCharacter OtherActor)
  (Variables|Default|SetbIsOpening false))

(event OnComponentBeginOverlap(ExitTrigger)
  (params (OverlappedComponent :type Primitive%20Component%20Object%20Reference) (OtherActor :type Actor%20Object%20Reference) (OtherComp :type Primitive%20Component%20Object%20Reference) (OtherBodyIndex :type Integer) (bFromSweep :type Boolean) (SweepResult :type Hit%20Result%20Structure%20%28by%20ref%29))
  (Utilities|Casting|CastToCharacter OtherActor)
  (if (Variables|Default|GetbIsFullyOpen)
    (Development|PrintString "Door")
    (else
      (Variables|Default|SetbInTrigger true))))

(event OnComponentEndOverlap(ExitTrigger)
  (params (OverlappedComponent :type Primitive%20Component%20Object%20Reference) (OtherActor :type Actor%20Object%20Reference) (OtherComp :type Primitive%20Component%20Object%20Reference) (OtherBodyIndex :type Integer))
  (Utilities|Casting|CastToCharacter OtherActor)
  (Variables|Default|SetbInTrigger false))

(event EventTick
  (params (DeltaSeconds :type Float%20%28single-precision%29))
  (bind _door (Variables|Default|GetDoor))
  (bind _relativelocation (Variables|/Script/Engine.SceneComponent|GetRelativeLocation _door))
  (if (Variables|Default|GetbIsOpening)
    (if (>= (.z _relativelocation) 2.2e+02)
      (Variables|Default|SetbIsFullyOpen true)
      (Variables|Default|SetbIsOpening false)
      (Variables|Default|SetNew%20Location (Math|Vector|MakeVector (.x _relativelocation) (.y _relativelocation) 2.2e+02))
      (if (Variables|Default|GetbInTrigger)
        (Development|PrintString "Door"))
      (else
        (Variables|Default|SetNew%20Location (Math|Vector|MakeVector (.x _relativelocation) (.y _relativelocation) (+ (.z _relativelocation) (* DeltaSeconds (Variables|Default|GetSpeed)))))
        (Transformation|SetRelativeLocation _door (Variables|Default|GetNew%20Location) false false)
        (Development|PrintString "Hello")))))

(fn ConstructionScript)