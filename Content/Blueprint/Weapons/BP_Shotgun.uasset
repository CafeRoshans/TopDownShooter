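; Shotgun weapon Blueprint that fires a spread of hitscan pellets toward the point under the mouse cursor.
; Fire spends a round from the magazine, or prints a message when empty, then aims from the muzzle at the cursor hit.
; Each pellet is a debug-drawn line trace along a random direction within the spread cone, dealing fixed damage to any BP_Target it hits.
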(event EventBeginPlay
  (|CallParentFunction) ; This node is disabled and will not be called.\nDrag off pins to build functionality.
)

(event Collision|EventActorBeginOverlap
  (params (OtherActor :type Actor%20Object%20Reference))
  (|CallParentFunction OtherActor) ; This node is disabled and will not be called.\nDrag off pins to build functionality.
)

(event EventTick
  (params (DeltaSeconds :type Float%20%28single-precision%29))
  (|CallParentFunction DeltaSeconds) ; This node is disabled and will not be called.\nDrag off pins to build functionality.
)

(event EventFire
  (bind _returnvalue (Game|GetPlayerController 0))
  (bind _muzzle (Variables|Default|GetMuzzle))
  (bind _returnvalue_2 (Transformation|GetWorldLocation _muzzle))
  (bind (_hitresult _returnvalue_3) (Game|Player|GetHitResultUnderCursorbyChannel _returnvalue "TraceTypeQuery1" false))
  (if (> (Variables|Default|GetAmmoInMag) 0)
    (Variables|Default|SetAmmoInMag (- (Variables|Default|GetAmmoInMag) 1))
    (if _returnvalue_3
      (for _index (range 0 (Variables|Default|GetPelletCount))
        (bind _outhit (Collision|LineTraceByChannel _returnvalue_2 (+ (* (Math|Random|RandomUnitVectorinConeinDegrees (Math|Vector|Normalize (- (.Location (Collision|BreakHitResult _hitresult)) _returnvalue_2)) (Variables|Default|GetSpreadAngle)) 5e+03) _returnvalue_2) "TraceTypeQuery1" false 0 "ForDuration"))
        (if (.bBlockingHit (Collision|BreakHitResult _outhit))
          (bind _asbp_target (Utilities|Casting|CastToBP_Target (.HitActor (Collision|BreakHitResult _outhit))))
          (Default|TakeDamage _asbp_target 25.0))))
    (else
      (Development|PrintString "No Ammo" true true "(R=1.000000,G=0.036223,B=0.000000,A=1.000000)"))))

(fn ConstructionScript
  (|CallParentFunction))