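; Base weapon Blueprint that provides Equip, Unequip, Fire and Reload events for weapons.
; Equip stores the owner, snaps the weapon mesh to its root component, shows it and fills the magazine.
; Fire only prints a should-be-overridden message, and Unequip is empty.
; Reload refills the magazine immediately and sets a non-looping timer bound to Reload itself, so it re-triggers after each ReloadTime.
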(event Custom|Equip
  (params (NewOwner :type Actor%20Object%20Reference))
  (bind _weaponmesh (Variables|Default|GetWeaponMesh))
  (bind _output_get (Variables|Default|SetWeaponOwner NewOwner))
  (Transformation|AttachComponentToComponent _weaponmesh (Variables|/Script/Engine.Actor|GetRootComponent _output_get) "None" "SnapToTarget" "SnapToTarget" "KeepRelative" true)
  (Rendering|SetVisibility _weaponmesh true false)
  (Variables|Main|SetAmmoInMag (Variables|Main|GetMagSize)))

(event Custom|Unequip)

(event Custom|Fire
  (Development|PrintString "Base Weapon Fire called - should be overridden!" true true "(R=1.000000,G=0.754670,B=0.000000,A=1.000000)"))

(event Custom|Reload
  (Utilities|Time|SetTimerbyEvent (delegate Custom|Reload) (Variables|Main|GetReloadTime))
  (Variables|Main|SetAmmoInMag (Variables|Main|GetMagSize)))

(event EventBeginPlay)

(event Collision|EventActorBeginOverlap
  (params (OtherActor :type Actor%20Object%20Reference)))

(event EventTick
  (params (DeltaSeconds :type Float%20%28single-precision%29)))

(fn ConstructionScript)